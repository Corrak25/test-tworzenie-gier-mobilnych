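; Zombie wave game mode that spawns enemies on begin play and advances the game through waves until the player wins.
; Each wave's zombie count scales with the wave number, split between two spawn locations.
; A kill counter triggers the next wave at zero, showing wave info on the first-person character and delaying before spawning.
; Clearing the final wave only prints a win message.
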(event `self.ReceiveBeginPlay`
  ;[1 1 1] Start Game
  (`self.Start Game`))

(event `Start Game`
  ;[1 1 1] Start Game
  (`self.Spawn Zombies`))

(event `Wave Start`
  ;[1 1 1] Start Next Wave
  (bind _asbp_first_person_character (cast `/Game/Assets/Blueprints/BP_FirstPersonCharacter` (`GameplayStatics.GetPlayerCharacter` 0)))
  (`/Game/Assets/Blueprints/BP_FirstPersonCharacter.Show Wave info` _asbp_first_person_character (`self.Current Wave`))
  (`KismetSystemLibrary.Delay` 5.0)
  (`self.Spawn Zombies`))

(event `Spawn Zombies`
  ;[1 1 1] Spawn Zombies
  (bind _output_get (set `self.Zombie Total` (* (`self.Current Wave`) 4)))
  (set `self.Zombies Left` _output_get)
  (for _index (range (+ _output_get 1))
    (if (== _index (/ (`self.Zombie Total`) 2))
      (break)
      (else
        (`|SpawnActorFromClass` "/Game/Assets/Enemies/Zombie/BP_Zombie.BP_Zombie_C" (`self.Spawn Location 1`) "Undefined" "OverrideRootScale" null null))))
  (for _ (range 1 (+ (/ (`self.Zombie Total`) 2) 1))
    (`|SpawnActorFromClass` "/Game/Assets/Enemies/Zombie/BP_Zombie.BP_Zombie_C" (`self.Spawn Location 2`) "Undefined" "OverrideRootScale" null null)))

(event `Zombie Killed`
  ;[1 1 1] Zombie Killed Counter
  (bind _result (`/Engine/EditorBlueprintResources/StandardMacros.DecrementInt` (`self.Zombies Left`))
    (:`  `
      (if (== _result 0)
        (`self.WAve Increment`)))))

(event `Wave Increment`
  ;[1 1 1] Update Wave
  (if (== (`self.Current Wave`) (`self.Max Waves`))
    (`KismetSystemLibrary.PrintString` "You win")
    (else
      (`/Engine/EditorBlueprintResources/StandardMacros.IncrementInt` (`self.Current Wave`)
        (:`  `
          (`self.Wave Start`))))))

(fn `UserConstructionScript`)